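; BP_Gravestone is a gravestone prop that randomizes its mesh, height offset, rotation and uniform scale for visual variety.
; ApplyAllVariations chains functions for each variation, bounded by Max variables, and picks a mesh from the NewMesh array.
; EventGraph events separately offer similar randomizers, with a full-circle yaw and a MeshVariations array.
; The construction script is empty, and nothing in the file triggers the randomization.
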(event Custom|Apply%20Random%20Z-Rotation
  (Transformation|SetRelativeRotation (Variables|Default|GetMesh) (Math|Rotator|MakeRotator 0.0 0.0 (Math|Random|RandomFloatinRange 0.0 3.6e+02)) false false))

(event Custom|Set%20Random%20Rotation
  (bind _maxrandomrotation (Variables|Default|GetMaxRandomRotation))
  (bind _returnvalue (* -1.0 _maxrandomrotation))
  (Transformation|SetRelativeRotation (Variables|Default|GetMesh) (Math|Rotator|MakeRotator (Math|Random|RandomFloatinRange _returnvalue _maxrandomrotation) (Math|Random|RandomFloatinRange _returnvalue _maxrandomrotation) (.yaw (Variables|/Script/Engine.SceneComponent|GetRelativeRotation (Variables|Default|GetMesh)))) false false))

(event Custom|RandomSizeVariation
  (bind _maxrandomsizevariation (Variables|Default|GetMaxRandomSizeVariation))
  (Transformation|SetRelativeScale3D (Variables|Default|GetMesh) (Math|Conversions|ToVector(Float) (+ (Math|Random|RandomFloatinRange (* _maxrandomsizevariation -1.0) _maxrandomsizevariation) 1.0))))

(event Custom|RandomMesh
  (Components|StaticMesh|SetStaticMesh (Variables|Default|GetMesh) (.OutItem (Utilities|Array|Random (Variables|Default|GetMeshVariations)))))

(fn ConstructionScript)

(fn RandomLocOffset
  (bind _maxheightoffset (Variables|Default|GetMaxHeightOffset))
  (Transformation|SetRelativeLocation (Variables|Default|GetMesh) (Math|Vector|MakeVector 0.0 0.0 (Math|Random|RandomFloatinRange (* _maxheightoffset -1.0) _maxheightoffset)) false false))

(fn RandomYaw
  (bind _mesh (Variables|Default|GetMesh))
  (bind _maxrandomyaw (Variables|Default|GetMaxRandomYaw))
  (bind _relativerotation (Variables|/Script/Engine.SceneComponent|GetRelativeRotation _mesh))
  (Transformation|SetRelativeRotation (Variables|Default|GetMesh) (Math|Rotator|MakeRotator (.roll _relativerotation) (.pitch _relativerotation) (Math|Random|RandomFloatinRange (* _maxrandomyaw -1.0) _maxrandomyaw)) false false))

(fn RandomRollandPitch
  (bind _maxrandomrotation (Variables|Default|GetMaxRandomRotation))
  (bind _maxrandomrotation_2 (Variables|Default|GetMaxRandomRotation))
  (Transformation|SetRelativeRotation (Variables|Default|GetMesh) (Math|Rotator|MakeRotator (Math|Random|RandomFloatinRange (* _maxrandomrotation_2 -1.0) _maxrandomrotation_2) (Math|Random|RandomFloatinRange (* _maxrandomrotation -1.0) _maxrandomrotation) (.yaw (Variables|/Script/Engine.SceneComponent|GetRelativeRotation (Variables|Default|GetMesh)))) false false))

(fn RandomScale
  (Transformation|SetRelativeScale3D (Variables|Default|GetMesh) (Math|Conversions|ToVector(Float) (Math|Random|RandomFloatinRange (- 1.0 (Variables|Default|GetMaxRandomSizeVariation)) (+ (Variables|Default|GetMaxRandomSizeVariation) 1.0)))))

(fn SetRandomMesh
  (Components|StaticMesh|SetStaticMesh (Variables|Default|GetMesh) (.OutItem (Utilities|Array|Random (Variables|Default|GetNew%20Mesh)))))

(fn ApplyAllVariations
  (CallFunction|RandomLocOffset)
  (CallFunction|RandomYaw)
  (CallFunction|RandomRollandPitch)
  (CallFunction|RandomScale)
  (CallFunction|SetRandomMesh))