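; Moving platform actor that travels along the spline of an assigned spline actor at a set speed, looping back to the start when it passes the end.
; Each tick it advances a distance along the spline and moves to that point, optionally matching only the spline's yaw.
; The construction script places it at a start fraction of the spline's length.
; An on-screen error prints once if no spline is assigned during the transform update.
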(event Custom|UpdateTransform
  (bind _splineactor (Variables|Default|GetSplineActor))
  (bind _distancealongspline (Variables|Default|GetDistanceAlongSpline))
  (bind _spline (Variables|/Game/BP/BP_Spline.BP_Spline_C|GetSpline _splineactor))
  (bind _returnvalue (Spline|GetTransformatDistanceAlongSpline _spline _distancealongspline "World" false))
  (Utilities|IsValid (Variables|Default|GetSplineActor)
    (:Is%20Valid
      (Transformation|SetActorLocation (.location _returnvalue) false false)
      (if (Variables|Default|GetbAlignRotationToSpline)
        (Transformation|SetActorRotation (Math|Rotator|MakeRotator 0.0 0.0 (.yaw (.rotation _returnvalue))))))
    (:Is%20Not%20Valid
      (Utilities|FlowControl|DoOnce false
        (:Completed
          (Development|PrintString "ERROR! Spline platform has no spline assigned!" true true "(R=1.000000,G=0.011454,B=0.000000,A=1.000000)" 5.0))))))

(event EventTick
  (params (DeltaSeconds :type Float%20%28single-precision%29))
  (CallFunction|UpdateDistanceAlongSpline)
  (CallFunction|UpdateTransform))

(event EventBeginPlay)

(fn ConstructionScript
  (CallFunction|SetStartDistance)
  (CallFunction|UpdateTransform))

(fn UpdateDistanceAlongSpline
  (bind _splineactor (Variables|Default|GetSplineActor))
  (bind _spline (Variables|/Game/BP/BP_Spline.BP_Spline_C|GetSpline _splineactor))
  (bind _returnvalue (Spline|GetSplineLength _spline))
  ;[0.15 0.15 0.15 0.5] Increase Distance
  (Variables|Default|SetDistanceAlongSpline (+ (Variables|Default|GetDistanceAlongSpline) (* (Variables|Default|GetSpeed) (Utilities|Time|GetWorldDeltaSeconds))))
  ;[0.15 0.15 0.15 0.5] Have we moved too far?
  (if (> (Variables|Default|GetDistanceAlongSpline) _returnvalue)
    ;[0.15 0.15 0.15 0.5] ... then start again
    (Variables|Default|SetDistanceAlongSpline (- (Variables|Default|GetDistanceAlongSpline) _returnvalue))))

(fn SetStartDistance
  (bind _splineactor (Variables|Default|GetSplineActor))
  (Utilities|IsValid _splineactor
    (:Is%20Valid
      (Variables|Default|SetDistanceAlongSpline (* (Spline|GetSplineLength (Variables|/Game/BP/BP_Spline.BP_Spline_C|GetSpline _splineactor)) (Variables|Default|GetDistanceOnStart))))))