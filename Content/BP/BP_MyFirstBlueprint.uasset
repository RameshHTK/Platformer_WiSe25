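; BP_MyFirstBlueprint is a practice actor with a transforming, rising mesh and a color-changing point light.
; BeginPlay calls ModifyMesh to offset, rotate, rescale and swap MyMesh to a pyramid.
; Tick moves the mesh upward frame-rate independently, then a Delay throttles RandomizeLight to roughly once per second, picking a preset color and ranged random intensity.
; AddFloats, the fully random color branch and the collision events are unused or empty.
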(event EventBeginPlay
  (CallFunction|ModifyMesh))

(event Collision|EventActorBeginOverlap
  (params (OtherActor :type Actor%20Object%20Reference))
  ;[0.15 0.15 0.15 0.5] Trigger and Collision
)

(event EventTick
  (params (DeltaSeconds :type Float%20%28single-precision%29))
  (CallFunction|MoveMesh DeltaSeconds)
  (Utilities|FlowControl|Delay 1.0)
  (CallFunction|RandomizeLight))

(event Collision|EventHit
  (params (MyComp :type Primitive%20Component%20Object%20Reference) (Other :type Actor%20Object%20Reference) (OtherComp :type Primitive%20Component%20Object%20Reference) (bSelfMoved :type Boolean) (HitLocation :type Vector :default "0, 0, 0") (HitNormal :type Vector :default "0, 0, 0") (NormalImpulse :type Vector :default "0, 0, 0") (Hit :type Hit%20Result%20Structure%20%28by%20ref%29))
  ;[0.15 0.15 0.15 0.5] Trigger and Collision
)

(fn ConstructionScript)

(fn RandomizeLight
  (Rendering|Components|Light|SetLightColor (Variables|Default|GetPointLight) (.OutItem (Utilities|Array|Random (Utilities|Array|MakeArray "(R=0.000000,G=0.974891,B=1.000000,A=1.000000)" "(R=0.004806,G=1.000000,B=0.023375,A=1.000000)" "(R=1.000000,G=0.013190,B=0.000000,A=1.000000)" "(R=1.000000,G=0.269505,B=0.000000,A=1.000000)"))) true)
  (Rendering|Components|Light|SetIntensity (Variables|Default|GetPointLight) (Math|Random|RandomFloatinRange (Variables|Default|GetLightIntensity_Min) (Variables|Default|GetLightIntensity_Max))))

(fn ModifyMesh
  (bind _mymesh (Variables|Default|GetMyMesh))
  (Transformation|AddWorldOffset _mymesh "0.000000,0.000000,100.000000" false false)
  (Transformation|AddWorldRotation _mymesh "0.000000,45.000000,0.000000" false false)
  (Transformation|SetWorldScale3D _mymesh "0.500000,0.500000,2.000000")
  (Components|StaticMesh|SetStaticMesh _mymesh "/ControlRig/Controls/ControlRig_Pyramid_3mm.ControlRig_Pyramid_3mm"))

(fn AddFloats
  (params (A :type Float%20%28double-precision%29) (B :type Float%20%28double-precision%29))
  (return (+ A B)))

(fn MoveMesh
  (params (DeltaSeconds :type Float%20%28single-precision%29))
  (Transformation|AddWorldOffset (Variables|Default|GetMyMesh) (* "0.000000,0.000000,20.000000" DeltaSeconds) false false))