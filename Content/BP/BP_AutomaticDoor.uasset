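; Automatic door that swings open when a BP_HTKCharacter enters its Box trigger and closes when it leaves.
; A Timeline drives Pivot yaw up to OpenAngle, playing on begin overlap and reversing on end overlap.
; Swing sign comes from the character's world location rotated into Box space via InverseTransformDirection, which ignores the door's position.
; CanChangeDirection locks that sign until the door fully closes.
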(event OnComponentEndOverlap(Box)
  (params (OverlappedComponent :type Primitive%20Component%20Object%20Reference) (OtherActor :type Actor%20Object%20Reference) (OtherComp :type Primitive%20Component%20Object%20Reference) (OtherBodyIndex :type Integer))
  (Utilities|Casting|CastToBP_HTKCharacter OtherActor)
  (bind (_direction _rotation) (Timeline|Timeline Reverse)
    (:Update
      (Transformation|SetRelativeRotation (Variables|Default|GetPivot) (Math|Rotator|MakeRotator 0.0 0.0 (* _rotation (Variables|Default|GetOpenAngle) (Variables|Default|GetDir))) false false))
    (:Finished
      (if (Utilities|Enum|Equal(Enum) _direction "Backward")
        (Variables|Default|SetCanChangeDirection true)))))

(event OnComponentBeginOverlap(Box)
  (params (OverlappedComponent :type Primitive%20Component%20Object%20Reference) (OtherActor :type Actor%20Object%20Reference) (OtherComp :type Primitive%20Component%20Object%20Reference) (OtherBodyIndex :type Integer) (bFromSweep :type Boolean) (SweepResult :type Hit%20Result%20Structure%20%28by%20ref%29))
  (bind _asbp_htkcharacter (Utilities|Casting|CastToBP_HTKCharacter OtherActor))
  (if (Variables|Default|GetCanChangeDirection)
    (Variables|Default|SetCanChangeDirection false)
    (Variables|Default|SetDir (Math|Float|SelectFloat -1.0 1.0 (> (.y (Math|Transform|InverseTransformDirection (Transformation|GetWorldTransform (Variables|Default|GetBox)) (Transformation|GetActorLocation _asbp_htkcharacter))) 0.0)))
    (bind (_direction _rotation) (Timeline|Timeline Play)
      (:Update
        (Transformation|SetRelativeRotation (Variables|Default|GetPivot) (Math|Rotator|MakeRotator 0.0 0.0 (* _rotation (Variables|Default|GetOpenAngle) (Variables|Default|GetDir))) false false))
      (:Finished
        (if (Utilities|Enum|Equal(Enum) _direction "Backward")
          (Variables|Default|SetCanChangeDirection true))))
    (else
      (Timeline|Timeline Play))))

(fn ConstructionScript)