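; BP_TimedSpikeTrap is a hazard that continuously extends and retracts spikes on a timed rhythm.
; The SpikeMovement timeline, play rate scaled by SpikeMoveDuration, drives the Pivot's relative Z up to MaxExtendDistance.
; A FlipFlop alternates forward and reverse playback, looping through MoveSpikes after DelayBetweenMovement.
; RhythmOffset delays the first move by a fraction of the full cycle, allowing staggered traps.
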(event Custom|MoveSpikes
  (Utilities|FlowControl|FlipFlop
    (:A
      (bind _extendp (Timeline|SpikeMovement PlayFromStart)
        (:Update
          (Transformation|SetRelativeLocation (Variables|Default|GetPivot) (Math|Vector|MakeVector 0.0 0.0 (* _extendp (Variables|Default|GetMaxExtendDistance))) false false))
        (:Finished
          (Utilities|FlowControl|Delay (Variables|Default|GetDelayBetweenMovement))
          (CallFunction|MoveSpikes))))
    (:B
      (Timeline|SpikeMovement ReverseFromEnd))))

(event EventBeginPlay
  (Components|Timeline|SetPlayRate (Variables|Default|GetSpikeMovement) (/ 1.0 (Variables|Default|GetSpikeMoveDuration)))
  (Utilities|FlowControl|Delay (* (* (+ (Variables|Default|GetSpikeMoveDuration) (Variables|Default|GetDelayBetweenMovement)) 2.0) (Variables|Default|GetRhythmOffset)))
  (CallFunction|MoveSpikes))

(fn ConstructionScript)