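; BP_CursedKirby is an enemy character with an "Angry" morph target that chases the player once they come within its sensing radius.
; Tick compares the player's distance against the SensingRadius sphere, using it as a range rather than relying on overlap events.
; A DoOnce starts an AIMoveTo toward the player, which re-issues itself a tick after each success or failure, so the chase never stops.
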(event Custom|StartChasingPlayer
  (AI|AIMoveTo self "0, 0, 0" (Game|Player|GetPlayerPawn 0) 5.0 false
    (:OnSuccess
      _)
    (:OnFail
      _))
  (Utilities|FlowControl|DelayUntilNextTick)
  (CallFunction|StartChasingPlayer))

(event EventBeginPlay
  (bind _mesh (Variables|Character|GetMesh))
  (Components|SkeletalMesh|SetMorphTarget (Components|SkeletalMesh|GetAnimInstance _mesh) "Angry" 1.0)
  (Components|SkeletalMesh|SetMorphTarget _mesh "Angry" 1.0 true))

(event EventTick
  (params (DeltaSeconds :type Float%20%28single-precision%29))
  (if (CallFunction|IsSensingPlayer)
    (Utilities|FlowControl|DoOnce false
      (:Completed
        (CallFunction|StartChasingPlayer)))))

(fn ConstructionScript)

(fn IsSensingPlayer
  (return (< (Math|Vector|VectorLength (- (Transformation|GetActorLocation (Game|Player|GetPlayerPawn 0)) (Transformation|GetWorldLocation (Variables|Default|GetSensingRadius)))) (Components|Sphere|GetScaledSphereRadius (Variables|Default|GetSensingRadius)))))